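; Base enemy actor that patrols back and forth at random speed and direction after a spawn timeline, whose lerp alpha is fixed at zero.
; Non-enemy hits reverse it; hitting the player deals damage and destroys it.
; Lost health or ramming leads to shared death logic: score, random pickup drop, explosion effects, camera shake.
; It increments the game mode's live-enemy count on spawn, decrementing only on damage deaths.
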(event `self.ReceiveTick`
  (params (DeltaSeconds :type "Float (single-precision)"))
  ;[1 1 1] Movement
  (if (`self.Move_enabled`)
    (`self.K2_SetActorLocation` (+ (`self.K2_GetActorLocation`) (* (`KismetMathLibrary.GreaterGreater_VectorRotator` (`KismetMathLibrary.MakeVector` 0.0 0.0 (* (`self.MoveSpeed`) (`KismetMathLibrary.SelectFloat` 1.0 -1.0 (`self.bMove_direction`))))) DeltaSeconds)) true)))

(event `self.ReceiveBeginPlay`
  (bind _spawnlocation (`self.SpawnLocation`))
  ;[1 1 1] Control Random Move Direction
  (bind _asbp_game_mod (cast `/Game/Blueprints/Misc/bpGameMod` (`GameplayStatics.GetGameMode`)))
  (bind _output_get (set `self.Bp_gameMod` _asbp_game_mod))
  (set `/Game/Blueprints/Misc/bpGameMod.LiveEnemies` (+ (`/Game/Blueprints/Misc/bpGameMod.LiveEnemies` _output_get) 1) _output_get)
  (set `self.bMove_direction` (`KismetMathLibrary.RandomBool`))
  (set `self.MoveSpeed` (`KismetMathLibrary.RandomFloatInRange` 800.0 1400.0))
  (set `self.SweepIn` (`KismetMathLibrary.RandomFloatInRange` 1200.0 1700.0))
  ;[1 1 1] Spawn Animation
  (set `self.SpawnLocation` (`self.K2_GetActorLocation`))
  (`Timeline|SpawnAnimation`
    (:`Update`
      (`self.K2_SetActorLocation` (`KismetMathLibrary.VLerp` _spawnlocation (- _spawnlocation (`KismetMathLibrary.MakeVector` 0.0 (`self.SweepIn`))))))
    (:`Finished`
      (set `self.Move_enabled` true))))

(event `self.ReceiveHit`
  (params (MyComp :type "PrimitiveComponent Object Reference") (Other :type "Actor Object Reference") (OtherComp :type "PrimitiveComponent Object Reference") (bSelfMoved :type Boolean) (HitLocation :type "Vector Structure") (HitNormal :type "Vector Structure") (NormalImpulse :type "Vector Structure") (Hit :type "HitResult Structure (by ref)"))
  (bind _pickups (`self.PickUps`))
  ;[1 1 1] Death
  (cast `/Game/Blueprints/Enemies/BpEnemyBase` Other
    (:`CastFailed`
      (set `self.bMove_direction` (not (`self.bMove_direction`)))
      (bind _asbp_player (cast `/Game/Blueprints/Misc/bpPlayer` Other))
      (`GameplayStatics.ApplyDamage` _asbp_player 50.0)
      (`/Game/Blueprints/Misc/bpGameMod.AddScore` (`self.Bp_gameMod`) :!label _label)
      (if (<= (`KismetMathLibrary.RandomFloatInRange` 0.0 1.0) (`self.DropRate`))
        (`|SpawnActorFromClass` (`|GetArrayItem` _pickups (`KismetMathLibrary.RandomIntegerInRange` 0 (`KismetArrayLibrary.Array_LastIndex` _pickups))) (`self.GetTransform`) "Undefined" "OverrideRootScale" null null))
      (`GameplayStatics.SpawnEmitterAtLocation` "/Game/Realistic_Starter_VFX_Pack_Vol2/Particles/Explosion/P_Explosion_Big_B.P_Explosion_Big_B" (`self.K2_GetActorLocation`))
      (`/Game/Blueprints/Misc/bpGameMod.CallCameShake` (`self.Bp_gameMod`) "/Game/Blueprints/Misc/bpCameraCheckExplosion.bpCameraCheckExplosion_C")
      (`GameplayStatics.PlaySound2D` "/Game/Audio/Explosion.Explosion" 1.0 1.0 0.0 null null)
      (`self.K2_DestroyActor`))))

(event `self.ReceiveAnyDamage`
  (params (Damage :type "Float (single-precision)") (DamageType :type "DamageType Object Reference") (InstigatedBy :type "Controller Object Reference") (DamageCauser :type "Actor Object Reference"))
  (bind _bp_gamemod (`self.Bp_gameMod`))
  ;[1 1 1] Death
  (set `self.Health` (`KismetMathLibrary.FClamp` (- (`self.Health`) Damage) 0.0 (`self.MaxHealth`)))
  (if (<= (`self.Health`) 0.0)
    (set `/Game/Blueprints/Misc/bpGameMod.LiveEnemies` (- (`/Game/Blueprints/Misc/bpGameMod.LiveEnemies` _bp_gamemod) 1) _bp_gamemod)
    (goto _label)))

(fn `UserConstructionScript`
  (set `self.Health` (`self.MaxHealth`)))