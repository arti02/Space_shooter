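; Enemy wave spawner that runs up to five sequential waves, each with its own enemy class list and count.
; A looping timer polls bpGameMod and starts the next wave once LiveEnemies is zero and WaveReady is set.
; BeginWave publishes the wave size to the game mode.
; SpawnWave spawns random classes in one loop at fixed X/Y with random Z, then sets WaveReady again.
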(event `self.ReceiveBeginPlay`
  ;[1 1 1] EventBeginPaly - Spawn Wave
  (bind _asbp_game_mod (cast `/Game/Blueprints/Misc/bpGameMod` (`GameplayStatics.GetGameMode`)))
  (set `self.bpGameMod` _asbp_game_mod)
  (bind _returnvalue (`KismetSystemLibrary.K2_SetTimer` null "WaveCheck" 0.5 true))
  (set `self.WaveTimer` _returnvalue))

(event `WaveCheck`
  (bind _output (`|GetArrayItem` (`self.WaveEnemyCount`) (`self.WaveIndex`)))
  ;[1 1 1] WaveCheck
  (if (and (== (`/Game/Blueprints/Misc/bpGameMod.LiveEnemies` (`self.bpGameMod`)) 0) (`self.bWaveReady`))
    (switch `int` (`self.WaveIndex`)
      (:`0`
        (`self.BeginWave` _output)
        (`self.SpawnWave` _output (`self.WavesEnemies1`)))
      (:`1`
        (`self.BeginWave` _output)
        (`self.SpawnWave` _output (`self.WavesEnemies2`)))
      (:`2`
        (`self.BeginWave` _output)
        (`self.SpawnWave` _output (`self.WavesEnemies3`)))
      (:`3`
        (`self.BeginWave` _output)
        (`self.SpawnWave` _output (`self.WavesEnemies4`)))
      (:`4`
        (`self.BeginWave` _output)
        (`self.SpawnWave` _output (`self.WavesEnemies5`))))
    (`/Engine/EditorBlueprintResources/StandardMacros.IncrementInt` (`self.WaveIndex`))))

(fn `BeginWave`
  (params (WaveTotal :type Integer))
  (bind _bpgamemod (`self.bpGameMod`))
  (set `self.bWaveReady` false)
  (set `self.WaveActive` 0)
  (set `/Game/Blueprints/Misc/bpGameMod.MaxWaves` WaveTotal _bpgamemod)
  (set `/Game/Blueprints/Misc/bpGameMod.ActiveWave` WaveTotal _bpgamemod))

(fn `SpawnWave`
  (params (WaveTotal :type Integer) (WaveEnemies :type "Array of /Game/Blueprints/Enemies/BpEnemyBase Class Reference"))
  (bind _bpgamemod (`self.bpGameMod`))
  (bind (_enemyspownlocationmin_x _enemyspownlocationmin_y _enemyspownlocationmin_z) (`KismetMathLibrary.BreakVector` (`/Game/Blueprints/Misc/bpGameMod.EnemySpownLocationMin` _bpgamemod)))
  (bind (_enemyspownlocationmax_x _enemyspownlocationmax_y _enemyspownlocationmax_z) (`KismetMathLibrary.BreakVector` (`/Game/Blueprints/Misc/bpGameMod.EnemySpownLocationMax` _bpgamemod)))
  (for _ (range (+ (+ WaveTotal 1) 1))
    (if (> WaveTotal (`self.WaveActive`))
      (if (not (`self.bWaveReady`))
        (`|SpawnActorFromClass` (`|GetArrayItem` WaveEnemies (`KismetMathLibrary.RandomInteger` (`KismetArrayLibrary.Array_Length` WaveEnemies))) (`KismetMathLibrary.MakeTransform` (`KismetMathLibrary.MakeVector` _enemyspownlocationmin_x _enemyspownlocationmin_y (`KismetMathLibrary.RandomFloatInRange` _enemyspownlocationmin_z _enemyspownlocationmax_z))) "AlwaysSpawn" "OverrideRootScale" null null)
        (set `self.WaveActive` (+ (`self.WaveActive`) 1)))
      (else
        (set `self.bWaveReady` true)))))

(fn `UserConstructionScript`)