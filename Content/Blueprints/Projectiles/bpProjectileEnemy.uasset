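; Enemy projectile actor that flies in its local space and damages the player on hit.
; Tick applies a swept local offset from Speed, and the construction script sets the actor's scale from a Scale variable.
; A mesh hit on bpPlayer applies damage, spawns a hit particle, triggers a camera shake through bpGameMod and destroys the projectile.
; Hits on other actors are ignored.
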(event `self.ReceiveTick`
  (params (DeltaSeconds :type "Float (single-precision)"))
  ;[1 1 1] Move Projectile
  (`self.K2_AddActorLocalOffset` (* (`self.Speed`) DeltaSeconds) true))

(event `self.StaticMesh.OnComponentHit`
  (params (HitComponent :type "PrimitiveComponent Object Reference") (OtherActor :type "Actor Object Reference") (OtherComp :type "PrimitiveComponent Object Reference") (NormalImpulse :type "Vector Structure") (Hit :type "HitResult Structure (by ref)"))
  ;[1 1 1] Collision Events
  (bind _asbp_player (cast `/Game/Blueprints/Misc/bpPlayer` OtherActor))
  (`GameplayStatics.ApplyDamage` _asbp_player (`self.Damage`))
  (`GameplayStatics.SpawnEmitterAtLocation` "/Game/Art/Particles/pHitEnemy.pHitEnemy" (`self.K2_GetActorLocation`))
  (bind _asbp_game_mod (cast `/Game/Blueprints/Misc/bpGameMod` (`GameplayStatics.GetGameMode`)))
  (`/Game/Blueprints/Misc/bpGameMod.CallCameShake` _asbp_game_mod "/Game/Blueprints/Misc/bpCameraShakeCollision.bpCameraShakeCollision_C")
  (`self.K2_DestroyActor`))

(fn `UserConstructionScript`
  (`self.SetActorScale3D` (`self.Scale`)))