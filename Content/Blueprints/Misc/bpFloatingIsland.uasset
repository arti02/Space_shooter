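; Floating island actor that drifts along negative world Y as moving scenery until it passes OffScreenLeft.
; Its construction script adds random tree meshes at three arrow-marked spawn points, randomizes scale per axis and applies a fixed tilt.
; Tick moves it a fixed step per frame, not scaled by delta time.
; Once past the limit, it stops, waits briefly, asks bpGameMod to spawn another island, then destroys itself.
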(event `self.ReceiveTick`
  (params (DeltaSeconds :type "Float (single-precision)"))
  (bind (_returnvalue_x _returnvalue_y) (`KismetMathLibrary.BreakVector` (`SceneComponent.K2_GetComponentLocation` (`self.Scene`))))
  (if (< _returnvalue_y (`self.OffScreenLeft`))
    (`KismetSystemLibrary.Delay` (`KismetMathLibrary.RandomFloatInRange` 1.0 2.0))
    (bind _asbp_game_mod (cast `/Game/Blueprints/Misc/bpGameMod` (`GameplayStatics.GetGameMode`)))
    (`/Game/Blueprints/Misc/bpGameMod.SpawnIsland` _asbp_game_mod)
    (`self.K2_DestroyActor`)
    (else
      (`self.K2_AddActorWorldOffset` (0.0 -20.0 0.0)))))

(fn `SetSpawnPoints`
  (set `self.spawnPoints` (`|MakeArray` (`SceneComponent.GetRelativeTransform` (`self.Arrow`)) (`SceneComponent.GetRelativeTransform` (`self.Arrow1`)) (`SceneComponent.GetRelativeTransform` (`self.Arrow2`)))))

(fn `SpawnTrees`
  (bind _spawnpoints (`self.spawnPoints`))
  (bind _trees (`self.Trees`))
  (for _index (range (`KismetArrayLibrary.Array_Length` _spawnpoints))
    (bind _returnvalue (`AddComponent|NODE_AddStaticMeshComponent-0` :`RelativeTransform` (`|GetArrayItem` _spawnpoints _index)))
    (`StaticMeshComponent.SetStaticMesh` _returnvalue (`|GetArrayItem` _trees (`KismetMathLibrary.RandomIntegerInRange` 0 (`KismetArrayLibrary.Array_LastIndex` _trees))))))

(fn `UserConstructionScript`
  (bind _returnvalue (`KismetMathLibrary.RandomFloatInRange` 0.3 1.0))
  (`self.SetSpawnPoints`)
  (`self.SpawnTrees`)
  (`self.SetActorScale3D` (`KismetMathLibrary.MakeVector` _returnvalue _returnvalue _returnvalue))
  (`self.K2_SetActorRotation` (struct :`Pitch` 15.0 :`Roll` -15.0)))