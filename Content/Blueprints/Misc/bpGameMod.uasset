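; Game mode Blueprint that tracks coins and score, persists the coin count, and provides island spawning and camera shake.
; Coins load from a bpCoinSave slot on BeginPlay, creating the save if absent, and save to a fresh object on EndPlay, which also calls Play on BGM.
; Helper functions increment coins and score or spawn a floating island at fixed X/Y with random height.
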(event `self.ReceiveBeginPlay`
  (`self.LoadCoins`))

(event `self.ReceiveEndPlay`
  (params (EndPlayReason :type "EEndPlayReason Enum" :default "Destroyed"))
  (`self.SaveCoins`)
  (`AudioComponent.Play` (`self.BGM`) 0.0))

(event `CallCameShake`
  (params (ShakeType :type "CameraShakeBase Class Reference"))
  (`GameplayStatics.PlayWorldCameraShake` ShakeType (0.0 0.0 0.0) -1.0 500.0))

(fn `AddCoin`
  (set `self.Coins` (+ (`self.Coins`) 1)))

(fn `AddScore`
  (set `self.Score` (+ (`self.Score`) 10)))

(fn `LoadCoins`
  (locals (NewLocalVar_0 :type String :default "Coins"))
  (bind _returnvalue (`GameplayStatics.DoesSaveGameExist` (`self.Coin Save Name`)))
  (if _returnvalue
    (bind _returnvalue_2 (`GameplayStatics.LoadGameFromSlot` (`self.Coin Save Name`)))
    (bind _output_get (set `self.Save Sub` _returnvalue_2))
    (bind _asbp_coin_save (cast `/Game/Blueprints/Misc/bpCoinSave` _output_get))
    (set `self.Coins` (`/Game/Blueprints/Misc/bpCoinSave.CoinCount` _asbp_coin_save))
    (`GameplayStatics.SaveGameToSlot` (`self.Save Sub`) (`self.Coin Save Name`))
    (else
      (`self.SaveCoins`))))

(fn `SaveCoins`
  (bind _returnvalue (`GameplayStatics.CreateSaveGameObject` "/Game/Blueprints/Misc/bpCoinSave.bpCoinSave_C"))
  (bind _output_get (set `self.Save Sub` _returnvalue))
  (bind _asbp_coin_save (cast `/Game/Blueprints/Misc/bpCoinSave` _output_get))
  (set `/Game/Blueprints/Misc/bpCoinSave.CoinCount` (`self.Coins`) _asbp_coin_save)
  (`GameplayStatics.SaveGameToSlot` (`self.Save Sub`) (`self.Coin Save Name`)))

(fn `SpawnIsland`
  (`|SpawnActorFromClass` "/Game/Blueprints/Misc/bpFloatingIsland.bpFloatingIsland_C" (`KismetMathLibrary.MakeTransform` (`KismetMathLibrary.MakeVector` 21000.0 35000.0 (`KismetMathLibrary.RandomFloatInRange` -2500.0 2500.0))) "AlwaysSpawn" "OverrideRootScale" null null)
  (`KismetSystemLibrary.PrintString` "Hello"))

(fn `UserConstructionScript`)